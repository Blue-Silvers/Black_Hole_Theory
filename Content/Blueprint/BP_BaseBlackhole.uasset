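; Base black hole actor with a configurable accretion disk look, gravitational lensing and an optional field of surrounding stars.
; The construction script pushes appearance variables into the Blackhole material and sets scale on two lensing shells, plus refraction on the outer one.
; ActivateStarsSpawn starts a near-per-frame timer that spawns randomly scaled BP_Star batches in a flattened, actor-scaled volume.
; Stars too close to the center are destroyed, and the timer pauses around 500 kept stars.
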(event Custom|SpawnStars
  (bind _returnvalue (Transformation|GetActorLocation))
  (bind _returnvalue_2 (Transformation|GetActorScale3D))
  (bind _returnvalue_3 (Math|Random|RandomFloatinRange 1.0 3.0))
  (bind _returnvalue_4 (Transformation|GetActorScale3D))
  (bind _returnvalue_5 (* _returnvalue_2 2e+02))
  (bind _returnvalue_6 (* (.x _returnvalue_4) 3e+01))
  (bind _returnvalue_7 (Math|Random|RandomPointinBoundingBox _returnvalue _returnvalue_5))
  ;[0.15 0.15 0.15 0.5] Spawn Star
  (for _index (range 1 10)
    (bind _returnvalue_8 (Game|SpawnActorfromClass "/Game/Blueprint/BP_Star.BP_Star_C" (Math|Transform|MakeTransform (Math|Vector|MakeVector (.x _returnvalue_7) (.y _returnvalue_7) (+ (.z (Transformation|GetWorldLocation (Variables|Default|GetBlackhole))) (Math|Random|RandomFloatinRange (* _returnvalue_6 -1.0) _returnvalue_6))) "0, 0, 0" (Math|Vector|MakeVector _returnvalue_3 _returnvalue_3 _returnvalue_3)) "Undefined" "MultiplyWithRoot" 0 0))
    (Utilities|IsValid _returnvalue_8
      (:Is%20Valid
        (if (> (Transformation|GetDistanceTo _returnvalue_8 self) (* (.x (Transformation|GetActorScale3D)) 5e+01))
          (bind _result (Math|Integer|IncrementInt (Variables|Default|GetstarCount))
            (:%20%20
              (if (>= _result 500)
                (Utilities|Time|PauseTimerbyHandle (Variables|Default|Gettimer)))))
          (else
            (Actor|DestroyActor _returnvalue_8)))))))

(event Custom|ActivateStarsSpawn
  (bind _returnvalue (Utilities|Time|SetTimerbyEvent (delegate Custom|SpawnStars) 0.0001 true true))
  (Variables|Default|Settimer _returnvalue))

(fn ConstructionScript
  ;[0.15 0.15 0.15 0.5] Blackhole settings
  (Rendering|Material|SetScalarParameterValueonMaterials (Variables|Default|GetBlackhole) "Blackhole_Size" (Variables|Blackhole|Global|GetBlackhole_Size))
  (Rendering|Material|SetVectorParameterValueonMaterials (Variables|Default|GetBlackhole) "Accreation_Disk_Color" (Variables|Blackhole|Disk|GetRing_Color))
  (Rendering|Material|SetScalarParameterValueonMaterials (Variables|Default|GetBlackhole) "Emission_Intensity" (Variables|Blackhole|Global|GetEmission_Intensity))
  (Rendering|Material|SetScalarParameterValueonMaterials (Variables|Default|GetBlackhole) "Ring_Speed" (Variables|Blackhole|Disk|GetRing_Speed))
  (Rendering|Material|SetScalarParameterValueonMaterials (Variables|Default|GetBlackhole) "Texture_Stretch" (Variables|Blackhole|Disk|GetTexture_Stretch))
  (Rendering|Material|SetScalarParameterValueonMaterials (Variables|Default|GetBlackhole) "Doppler_Intensity" (Variables|Blackhole|Doppler|GetDoppler_Intensity))
  (Rendering|Material|SetScalarParameterValueonMaterials (Variables|Default|GetBlackhole) "Event_Horizon_size" (Variables|Blackhole|Hole|GetEvent_Horizon_size))
  ;[0.15 0.15 0.15 0.5] Gravitational lensing
  (Transformation|SetRelativeScale3D (Variables|Default|GetOuter_Lensing) (Variables|Blackhole|Doppler|GetLensing_Scale))
  (Rendering|Material|SetScalarParameterValueonMaterials (Variables|Default|GetOuter_Lensing) "Fresnel_Intensity" (Variables|Blackhole|Doppler|GetRefraction_Intensity))
  (Rendering|Material|SetScalarParameterValueonMaterials (Variables|Default|GetOuter_Lensing) "Refraction_Power" (Variables|Blackhole|Doppler|GetRefraction_Power))
  (Transformation|SetRelativeScale3D (Variables|Default|GetIner_Lensing) (* (Variables|Blackhole|Doppler|GetLensing_Scale) 0.7)))
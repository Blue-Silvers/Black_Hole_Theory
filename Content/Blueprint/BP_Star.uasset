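; BP_Star is a star actor that shows a randomly colored plane and slowly turns to face the player.
; The construction script gives the plane a dynamic M_Star material with a random bright Color, capping green and blue by subtracting random draws from a shared maximum.
; A looping timer, rather than Tick, interpolates the root's rotation toward the player pawn's location.
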(event Custom|RotateStar
  (bind _defaultsceneroot (Variables|Default|GetDefaultSceneRoot))
  (Transformation|SetWorldRotation _defaultsceneroot (Math|Interpolation|RInterpTo (Transformation|GetWorldRotation _defaultsceneroot) (Math|Rotator|FindLookatRotation (Transformation|GetActorLocation) (Transformation|GetActorLocation (Game|Player|GetPlayerPawn 0))) (Utilities|Time|GetWorldDeltaSeconds) 1.0) false false))

(event EventBeginPlay
  (Utilities|Time|SetTimerbyEvent (delegate Custom|RotateStar) 0.2 true true))

(event EventTick
  (params (DeltaSeconds :type Float%20%28single-precision%29)))

(fn ConstructionScript
  (bind _returnvalue (Math|Random|RandomFloatinRange 1.0 1e+02))
  (bind _returnvalue_2 (- 1e+02 _returnvalue))
  (bind _returnvalue_3 (Math|Float|Clamp(Float) _returnvalue_2 1.0 1e+02))
  (bind _returnvalue_4 (Math|Random|RandomFloatinRange 1.0 _returnvalue_3))
  (bind _returnvalue_5 (Rendering|Material|CreateDynamicMaterialInstance "/Game/Material/M_Star.M_Star" "None" "None" :!class /Script/Engine.KismetMaterialLibrary))
  (Rendering|Material|SetMaterial (Variables|Default|GetPlane) 0 _returnvalue_5)
  (Rendering|Material|SetVectorParameterValue _returnvalue_5 "Color" (Utilities|Struct|MakeLinearColor _returnvalue _returnvalue_4 (Math|Float|Clamp(Float) (- _returnvalue_2 _returnvalue_4) 1.0 1e+02) 1.0) :!class /Script/Engine.MaterialInstanceDynamic))